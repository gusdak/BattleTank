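; AutoMortar_BP is a mortar with a health bar that passes its Barrel and Dome to a TankAiming component on BeginPlay.
; BeginPlay also sets current health to the starting value and hands the mortar to its HealthBar widget.
; AnyDamage subtracts damage through a math expression and truncates the result, while GetHealthPercentage returns current over starting health as a fraction.
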(event EventBeginPlay
  (Class|TankAimingComponent|Inintitalize (Variables|Default|GetTankAiming) (Variables|Default|GetBarrel) (Variables|Default|GetDome))
  (CallFunction|InitializeHealthBarWidget))

(event Game|Damage|EventAnyDamage
  (params (Damage :type Float%20%28single-precision%29) (DamageType :type Damage%20Type%20Object%20Reference) (InstigatedBy :type Controller%20Object%20Reference) (DamageCauser :type Actor%20Object%20Reference))
  (Variables|Default|SetCurrentHealth (Math|Float|Truncate (|({F15BEDF2-46AA-8845-796D-69813E98C30A}-Damage) Damage))))

(fn ConstructionScript)

(fn InitializeHealthBarWidget
  (Variables|Default|SetCurrentHealth (Variables|Default|GetStartingHealth))
  (bind _ashealth_bar (Utilities|Casting|CastToHealthBar (UserInterface|GetUserWidgetObject (Variables|Default|GetWidget))))
  (Variables|/Game/UI/HealthBar.HealthBar_C|SetMyMortar _ashealth_bar self))

(fn GetHealthPercentage
  (return (|(CH/SH) (Math|Conversions|ToFloat(Integer) (Variables|Default|GetStartingHealth)) (Math|Conversions|ToFloat(Integer) (Variables|Default|GetCurrentHealth)))))